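; Interactable incinerator that destroys the gathered materials to bring up the game-complete screen.
; A trigger box toggles an interaction icon as overlaps begin and end.
; Interact checks the PlayerGamemode's materials-acquired flag, showing a needs-materials widget when unset.
; When set, it calls the incinerator event, plays an explosion effect and sound, adds the completion widget and advances the current objective.
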(event OnComponentBeginOverlap(Box)
  (params (OverlappedComponent :type Primitive%20Component%20Object%20Reference) (OtherActor :type Actor%20Object%20Reference) (OtherComp :type Primitive%20Component%20Object%20Reference) (OtherBodyIndex :type Integer) (bFromSweep :type Boolean) (SweepResult :type Hit%20Result%20Structure%20%28by%20ref%29))
  (Development|SetHiddeninGame (Variables|Default|GetInteractIcon) false false))

(event OnComponentEndOverlap(Box)
  (params (OverlappedComponent :type Primitive%20Component%20Object%20Reference) (OtherActor :type Actor%20Object%20Reference) (OtherComp :type Primitive%20Component%20Object%20Reference) (OtherBodyIndex :type Integer))
  (Development|SetHiddeninGame (Variables|Default|GetInteractIcon) true false))

(event Custom|DestroyMaterials
  (Default|CallIncineratorEvent)
  (Effects|SpawnEmitteratLocation "/Game/Assets/StarterContent/Particles/P_Explosion.P_Explosion" (Transformation|GetWorldLocation (Variables|Default|GetIncinerator)) "0, 0, 0" "2.000000,2.000000,2.000000")
  (bind _returnvalue (UserInterface|CreateWidget "/Game/Game/Widgets/GameCompleteScreen.GameCompleteScreen_C"))
  (UserInterface|Viewport|AddtoViewport _returnvalue 0)
  (Audio|PlaySoundatLocation "/Game/Assets/StarterContent/Audio/Explosion02.Explosion02" (Transformation|GetWorldLocation (Variables|Default|GetParticleSystem)) "0, 0, 0" 1.0 1.0 0.0 0 0 0))

(fn ConstructionScript)

(fn Interact
  (params (Interacting%20Entity :type Character%20Object%20Reference))
  (bind _asplayer_gamemode (Utilities|Casting|CastToPlayerGamemode (Game|GetGameMode)))
  (if (Variables|/Game/Game/Player/PlayerGamemode.PlayerGamemode_C|GetMaterialsAquired? _asplayer_gamemode)
    (CallFunction|DestroyMaterials)
    (Variables|/Game/Game/Player/PlayerGamemode.PlayerGamemode_C|SetCurrentObjective _asplayer_gamemode 10)
    (else
      (bind _returnvalue (UserInterface|CreateWidget "/Game/Game/Widgets/Hints/NeedsMaterials.NeedsMaterials_C"))
      (UserInterface|Viewport|AddtoViewport _returnvalue 0)))
  (return false))