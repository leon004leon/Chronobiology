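; CeilingLight1_BP is a ceiling light with configurable intensity, attenuation radius, color temperature and shadow casting.
; The construction script applies those settings to its PointLight component.
; When IsFlickering is set, Tick runs through a short random Delay into a FlipFlop, alternating between full intensity and a random lower one to produce the flicker.
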(event EventBeginPlay)

(event Collision|EventActorBeginOverlap
  (params (OtherActor :type Actor%20Object%20Reference)))

(event EventTick
  (params (DeltaSeconds :type Float%20%28single-precision%29))
  (if (Variables|Default|GetIsFlickering?)
    (Utilities|FlowControl|Delay (Math|Random|RandomFloatinRange 0.05 0.1))
    (Utilities|FlowControl|FlipFlop
      (:A
        (Rendering|Components|Light|SetIntensity (Variables|Default|GetPointLight) (Variables|Default|GetLightIntensity)))
      (:B
        (Rendering|Components|Light|SetIntensity (Variables|Default|GetPointLight) (Math|Random|RandomFloatinRange 5.0 (Variables|Default|GetLightIntensity)))))))

(fn ConstructionScript
  (bind _pointlight (Variables|Default|GetPointLight))
  (Utilities|FlowControl|Sequence
    (:then_0
      (Rendering|Components|Light|SetIntensity _pointlight (Variables|Default|GetLightIntensity)))
    (:then_1
      (Rendering|Lighting|SetAttenuationRadius _pointlight (Variables|Default|GetAttenuationRadius)))
    (:then_2
      (Class|LightComponent|SetTemperature _pointlight (Variables|Default|GetLightTemp)))
    (:then_3
      (if (Variables|Default|GetCastShadows?)
        (Rendering|Components|Light|SetCastShadows _pointlight true)
        (else
          (Rendering|Components|Light|SetCastShadows _pointlight false))))))