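; An interactable safe that the player blows open, then loots for quest materials.
; The first Interact swaps in the open mesh with an explosion effect and sound; a later one, gated by DoOnce, collects the materials.
; Collection destroys the Materials component, flags PlayerGamemode, shows a notification widget and sets the current objective.
; A collider overlap toggles the interact prompt, checking InteractIteration before showing it.
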(event OnComponentBeginOverlap(SafeCollider)
  (params (OverlappedComponent :type Primitive%20Component%20Object%20Reference) (OtherActor :type Actor%20Object%20Reference) (OtherComp :type Primitive%20Component%20Object%20Reference) (OtherBodyIndex :type Integer) (bFromSweep :type Boolean) (SweepResult :type Hit%20Result%20Structure%20%28by%20ref%29))
  (if (< (Variables|Default|GetInteractIteration) 2)
    (Development|SetHiddeninGame (Variables|Default|GetInteractPrompt) false false)))

(event OnComponentEndOverlap(SafeCollider)
  (params (OverlappedComponent :type Primitive%20Component%20Object%20Reference) (OtherActor :type Actor%20Object%20Reference) (OtherComp :type Primitive%20Component%20Object%20Reference) (OtherBodyIndex :type Integer))
  (Development|SetHiddeninGame (Variables|Default|GetInteractPrompt) true false))

(event Custom|Safe%20Explode
  (bind _safe (Variables|Default|GetSafe))
  (bind _returnvalue (Transformation|GetWorldLocation _safe))
  (Components|StaticMesh|SetStaticMesh _safe "/Game/Assets/Models/SafeOpen.SafeOpen")
  (Effects|SpawnEmitteratLocation "/Game/Assets/StarterContent/Particles/P_Explosion.P_Explosion" _returnvalue)
  (Audio|PlaySoundatLocation "/Game/Assets/StarterContent/Audio/Explosion01.Explosion01" _returnvalue "0, 0, 0" 1.0 1.0 0.0 0 0 0)
  (Variables|Default|SetInteractIteration 1))

(event Custom|Materials%20Aquired
  (Components|DestroyComponent (Variables|Default|GetMaterials))
  (bind _asplayer_gamemode (Utilities|Casting|CastToPlayerGamemode (Game|GetGameMode)))
  (Variables|/Game/Game/Player/PlayerGamemode.PlayerGamemode_C|SetMaterialsAquired? _asplayer_gamemode true)
  (bind _returnvalue (UserInterface|CreateWidget "/Game/Game/Widgets/Hints/MaterialsAquired.MaterialsAquired_C"))
  (UserInterface|Viewport|AddtoViewport _returnvalue 0)
  (Variables|/Game/Game/Player/PlayerGamemode.PlayerGamemode_C|SetCurrentObjective _asplayer_gamemode 9))

(event EventBeginPlay)

(event Collision|EventActorBeginOverlap
  (params (OtherActor :type Actor%20Object%20Reference)))

(event EventTick
  (params (DeltaSeconds :type Float%20%28single-precision%29)))

(fn ConstructionScript)

(fn Interact
  (params (Interacting%20Entity :type Character%20Object%20Reference))
  (if (== (Variables|Default|GetInteractIteration) 0)
    (CallFunction|SafeExplode)
    (else
      (Utilities|FlowControl|DoOnce false
        (:Completed
          (CallFunction|MaterialsAquired)))))
  (return false))