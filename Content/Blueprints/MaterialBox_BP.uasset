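; MaterialBox is an interactable actor that explodes and brings up the game complete screen when interacted with.
; Overlapping its Box component shows a Widget component, and ending the overlap hides it, with no check on the overlapping actor.
; Interact calls a custom Destroy event, which spawns an explosion, destroys only the Material component rather than the actor, and adds GameCompleteScreen to the viewport.
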(event OnComponentBeginOverlap(Box)
  (params (OverlappedComponent :type Primitive%20Component%20Object%20Reference) (OtherActor :type Actor%20Object%20Reference) (OtherComp :type Primitive%20Component%20Object%20Reference) (OtherBodyIndex :type Integer) (bFromSweep :type Boolean) (SweepResult :type Hit%20Result%20Structure%20%28by%20ref%29))
  (Development|SetHiddeninGame (Variables|Default|GetWidget) false false))

(event OnComponentEndOverlap(Box)
  (params (OverlappedComponent :type Primitive%20Component%20Object%20Reference) (OtherActor :type Actor%20Object%20Reference) (OtherComp :type Primitive%20Component%20Object%20Reference) (OtherBodyIndex :type Integer))
  (Development|SetHiddeninGame (Variables|Default|GetWidget) true false))

(event Custom|Destroy
  (bind _material (Variables|Default|GetMaterial))
  (Effects|SpawnEmitteratLocation "/Game/Assets/StarterContent/Particles/P_Explosion.P_Explosion" (Transformation|GetSocketLocation _material "None"))
  (Components|DestroyComponent _material)
  (bind _returnvalue (UserInterface|CreateWidget "/Game/Game/Widgets/GameCompleteScreen.GameCompleteScreen_C"))
  (UserInterface|Viewport|AddtoViewport _returnvalue 0))

(event EventBeginPlay)

(event Collision|EventActorBeginOverlap
  (params (OtherActor :type Actor%20Object%20Reference)))

(event EventTick
  (params (DeltaSeconds :type Float%20%28single-precision%29)))

(fn ConstructionScript)

(fn Interact
  (params (Interacting%20Entity :type Character%20Object%20Reference))
  (CallFunction|Destroy)
  (return false))