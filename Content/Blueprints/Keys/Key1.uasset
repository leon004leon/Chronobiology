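; Key1 is an interactable key pickup actor that records the first key as collected.
; Collider overlaps show and hide an InteractWidget prompt, without filtering which actor overlaps.
; Interact calls PickupKey, which sets the Key1 flag on PlayerGamemode and destroys the actor, so key state lives in the game mode.
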(event OnComponentBeginOverlap(Collider)
  (params (OverlappedComponent :type Primitive%20Component%20Object%20Reference) (OtherActor :type Actor%20Object%20Reference) (OtherComp :type Primitive%20Component%20Object%20Reference) (OtherBodyIndex :type Integer) (bFromSweep :type Boolean) (SweepResult :type Hit%20Result%20Structure%20%28by%20ref%29))
  (Development|SetHiddeninGame (Variables|Default|GetInteractWidget) false false))

(event OnComponentEndOverlap(Collider)
  (params (OverlappedComponent :type Primitive%20Component%20Object%20Reference) (OtherActor :type Actor%20Object%20Reference) (OtherComp :type Primitive%20Component%20Object%20Reference) (OtherBodyIndex :type Integer))
  (Development|SetHiddeninGame (Variables|Default|GetInteractWidget) true false))

(event Custom|PickupKey
  (bind _asplayer_gamemode (Utilities|Casting|CastToPlayerGamemode (Game|GetGameMode)))
  (Variables|/Game/Game/Player/PlayerGamemode.PlayerGamemode_C|SetKey1? _asplayer_gamemode true)
  (Actor|DestroyActor))

(fn ConstructionScript)

(fn Interact
  (params (Interacting%20Entity :type Character%20Object%20Reference))
  (CallFunction|PickupKey)
  (return false))