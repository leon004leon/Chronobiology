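; Control panel door Blueprint that opens a pair of door panels once the control panel is unlocked in the PlayerGamemode.
; Tick polls the game mode's ControlPanelUnlocked flag and, through a DoOnce, fires the OpenDoor event a single time.
; OpenDoor plays the DoorOpen timeline, which lerps both panels' relative Z upward to raise them, keeping their opposite X offsets fixed.
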(event Custom|OpenDoor
  (bind _dooropen (Timeline|DoorOpen Play)
    (:Update
      (Transformation|SetRelativeLocation (Variables|Default|GetDoor) (Math|Vector|MakeVector -162.5 0.0 (Math|Float|Lerp 0.0 3e+02 _dooropen)) false false)
      (Transformation|SetRelativeLocation (Variables|Default|GetDoor1) (Math|Vector|MakeVector 162.5 0.0 (Math|Float|Lerp 0.0 3e+02 _dooropen)) false false))))

(event EventTick
  (params (DeltaSeconds :type Float%20%28single-precision%29))
  (bind _asplayer_gamemode (Utilities|Casting|CastToPlayerGamemode (Game|GetGameMode)))
  (if (Variables|/Game/Game/Player/PlayerGamemode.PlayerGamemode_C|GetControlPanelUnlocked? _asplayer_gamemode)
    (Utilities|FlowControl|DoOnce false
      (:Completed
        (CallFunction|OpenDoor)))))

(fn ConstructionScript)