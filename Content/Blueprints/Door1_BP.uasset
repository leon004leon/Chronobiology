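; Interactable double door that swings both leaves open or closed and can require one of two keys.
; A timeline lerps each leaf's yaw and flips IsOpen on finishing, while an overlap component shows a widget near the closed door.
; Interact checks Interactable and the game mode's key flags, showing unlocked, key-required or uninteractable UI through DoOnce nodes.
; The unlocked DoOnce also gates the keyed toggle, so that path fires only once.
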(event OnComponentBeginOverlap(DoorInteractDistance)
  (params (OverlappedComponent :type Primitive%20Component%20Object%20Reference) (OtherActor :type Actor%20Object%20Reference) (OtherComp :type Primitive%20Component%20Object%20Reference) (OtherBodyIndex :type Integer) (bFromSweep :type Boolean) (SweepResult :type Hit%20Result%20Structure%20%28by%20ref%29))
  (if (not (Variables|Default|GetIsOpen?))
    (Development|SetHiddeninGame (Variables|Default|GetWidget) false false)))

(event OnComponentEndOverlap(DoorInteractDistance)
  (params (OverlappedComponent :type Primitive%20Component%20Object%20Reference) (OtherActor :type Actor%20Object%20Reference) (OtherComp :type Primitive%20Component%20Object%20Reference) (OtherBodyIndex :type Integer))
  (Development|SetHiddeninGame (Variables|Default|GetWidget) true false))

(event Custom|CloseDoor
  (bind _dooropenclose (Timeline|DoorOpenClose Reverse)
    (:Update
      (Transformation|SetRelativeRotation (Variables|Default|GetDoorRight) (Math|Rotator|MakeRotator 0.0 0.0 (Math|Float|Lerp (Variables|Default|GetDoorRightClosedRotation) (Variables|Default|GetDoorRightOpenRotation) _dooropenclose)) false false)
      (Transformation|SetRelativeRotation (Variables|Default|GetDoorLeft) (Math|Rotator|MakeRotator 0.0 0.0 (Math|Float|Lerp (Variables|Default|GetDoorLeftClosedRotation) (Variables|Default|GetDoorLeftOpenRotation) _dooropenclose)) false false))
    (:Finished
      (Variables|Default|SetIsOpen? (not (Variables|Default|GetIsOpen?))))))

(event Custom|OpenDoor
  (Development|SetHiddeninGame (Variables|Default|GetWidget) true false)
  (bind _dooropenclose (Timeline|DoorOpenClose Play)
    (:Update
      (Transformation|SetRelativeRotation (Variables|Default|GetDoorRight) (Math|Rotator|MakeRotator 0.0 0.0 (Math|Float|Lerp (Variables|Default|GetDoorRightClosedRotation) (Variables|Default|GetDoorRightOpenRotation) _dooropenclose)) false false)
      (Transformation|SetRelativeRotation (Variables|Default|GetDoorLeft) (Math|Rotator|MakeRotator 0.0 0.0 (Math|Float|Lerp (Variables|Default|GetDoorLeftClosedRotation) (Variables|Default|GetDoorLeftOpenRotation) _dooropenclose)) false false))
    (:Finished
      (Variables|Default|SetIsOpen? (not (Variables|Default|GetIsOpen?))))))

(fn ConstructionScript)

(fn Interact
  (params (Interacting%20Entity :type Character%20Object%20Reference))
  ;[1 1 1] Is Interactable?
  (if (Variables|Default|GetInteractable?)
    ;[1 1 1] Key required?
    (if (Variables|Default|GetKeyRequired?)
      ;[1 1 1] Y
      (bind _asplayer_gamemode (Utilities|Casting|CastToPlayerGamemode (Game|GetGameMode)))
      (switch int (Variables|Default|GetKeyNumber)
        (:0
          (if (Variables|/Game/Game/Player/PlayerGamemode.PlayerGamemode_C|GetKey0? _asplayer_gamemode)
            (Utilities|FlowControl|DoOnce false :!label _label
              (:Completed
                (bind _returnvalue (UserInterface|CreateWidget "/Game/Game/Widgets/Hints/Door_Unlocked.Door_Unlocked_C"))
                (UserInterface|Viewport|AddtoViewport _returnvalue 0)
                ;[1 1 1] N
                (if (not (Variables|Default|GetIsOpen?)) :!label _label_2
                  (CallFunction|OpenDoor)
                  (else
                    (CallFunction|CloseDoor)))
                (return true)))
            (else
              _)))
        (:1
          (if (Variables|/Game/Game/Player/PlayerGamemode.PlayerGamemode_C|GetKey1? _asplayer_gamemode)
            (goto _label)
            (else
              _))))
      (Utilities|FlowControl|DoOnce false
        (:Completed
          (bind _returnvalue_2 (UserInterface|CreateWidget "/Game/Game/Widgets/Hints/Door_KeyRequired.Door_KeyRequired_C"))
          (UserInterface|Viewport|AddtoViewport _returnvalue_2 0)))
      (else
        (goto _label_2)))
    (else
      (Utilities|FlowControl|DoOnce false
        (:Completed
          (bind _returnvalue_3 (UserInterface|CreateWidget "/Game/Game/Widgets/Hints/Door_Uninteractable.Door_Uninteractable_C"))
          (UserInterface|Viewport|AddtoViewport _returnvalue_3 0))))))