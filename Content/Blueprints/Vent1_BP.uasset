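; Interactable vent that moves the player character to a preset target location when used.
; Interact fires VentInteract, where the VentOpen timeline lerps the mesh pitch from closed to open, then sets player 0's location without sweep.
; VentClose then plays in reverse, updating the same rotation node, which reads VentOpen's track.
; Collider overlap begin and end show and hide the interact widget.
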(event OnComponentBeginOverlap(Collider)
  (params (OverlappedComponent :type Primitive%20Component%20Object%20Reference) (OtherActor :type Actor%20Object%20Reference) (OtherComp :type Primitive%20Component%20Object%20Reference) (OtherBodyIndex :type Integer) (bFromSweep :type Boolean) (SweepResult :type Hit%20Result%20Structure%20%28by%20ref%29))
  (Development|SetHiddeninGame (Variables|Default|GetInteractWidget) false false))

(event OnComponentEndOverlap(Collider)
  (params (OverlappedComponent :type Primitive%20Component%20Object%20Reference) (OtherActor :type Actor%20Object%20Reference) (OtherComp :type Primitive%20Component%20Object%20Reference) (OtherBodyIndex :type Integer))
  (Development|SetHiddeninGame (Variables|Default|GetInteractWidget) true false))

(event Custom|VentInteract
  (bind _ventopenclose (Timeline|VentOpen Play)
    (:Update
      _)
    (:Finished
      (Transformation|SetActorLocation (Game|GetPlayerCharacter 0) (Variables|Default|GetPlayerTargetLocation) false false)
      (Timeline|VentClose Reverse
        (:Update
          _))))
  (Transformation|SetRelativeRotation (Variables|Default|GetStaticMesh) (Math|Rotator|MakeRotator 0.0 (Math|Float|Lerp (Variables|Default|GetClosedRotation) (Variables|Default|GetOpenRotation) _ventopenclose) 0.0) false false))

(fn ConstructionScript)

(fn Interact
  (params (Interacting%20Entity :type Character%20Object%20Reference))
  (CallFunction|VentInteract)
  (return false))