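; One-shot interactable lift that rises along Z when used.
; An overlap box shows a prompt widget until the lift has been used and hides it on exit.
; Interact sets the Interacted flag, hides the widget, fires the lift-up sequence call and starts a timeline that lerps the Lift component between two fixed heights.
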(event OnComponentBeginOverlap(Box)
  (params (OverlappedComponent :type Primitive%20Component%20Object%20Reference) (OtherActor :type Actor%20Object%20Reference) (OtherComp :type Primitive%20Component%20Object%20Reference) (OtherBodyIndex :type Integer) (bFromSweep :type Boolean) (SweepResult :type Hit%20Result%20Structure%20%28by%20ref%29))
  (if (not (Variables|Default|GetInteracted?))
    (CallFunction|WidgetVisibile)))

(event OnComponentEndOverlap(Box)
  (params (OverlappedComponent :type Primitive%20Component%20Object%20Reference) (OtherActor :type Actor%20Object%20Reference) (OtherComp :type Primitive%20Component%20Object%20Reference) (OtherBodyIndex :type Integer))
  (CallFunction|WidgetHidden))

(event Custom|LiftUp
  (bind _liftup (Timeline|LiftUpTime Play)
    (:Update
      (Transformation|SetRelativeLocation (Variables|Default|GetLift) (Math|Vector|MakeVector 0.0 0.0 (Math|Float|Lerp 128.0 9.1e+02 _liftup)) false false))))

(fn ConstructionScript)

(fn WidgetVisibile
  (Development|SetHiddeninGame (Variables|Default|GetWidget) false false))

(fn WidgetHidden
  (Development|SetHiddeninGame (Variables|Default|GetWidget) true false))

(fn Interact
  (params (Interacting%20Entity :type Character%20Object%20Reference))
  (if (not (Variables|Default|GetInteracted?))
    (Variables|Default|SetInteracted? true)
    (CallFunction|WidgetHidden)
    (CallFunction|LiftUp)
    (Default|CallLiftUpSequence)
    (return false)))