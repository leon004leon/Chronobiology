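; Interactable control panel that, once used with the first key, flags itself unlocked in PlayerGamemode and advances the current objective.
; A box trigger shows the interact prompt until the panel has been used and hides it on exit.
; Interact checks the game mode's Key1 flag, shows a key-required, unlocked or already-used widget, and calls OpenDoor on first success to update the game mode.
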(event OnComponentBeginOverlap(Box)
  (params (OverlappedComponent :type Primitive%20Component%20Object%20Reference) (OtherActor :type Actor%20Object%20Reference) (OtherComp :type Primitive%20Component%20Object%20Reference) (OtherBodyIndex :type Integer) (bFromSweep :type Boolean) (SweepResult :type Hit%20Result%20Structure%20%28by%20ref%29))
  (if (not (Variables|Default|GetInteracted?))
    (Development|SetHiddeninGame (Variables|Default|GetInteractWidget) false false)))

(event OnComponentEndOverlap(Box)
  (params (OverlappedComponent :type Primitive%20Component%20Object%20Reference) (OtherActor :type Actor%20Object%20Reference) (OtherComp :type Primitive%20Component%20Object%20Reference) (OtherBodyIndex :type Integer))
  (Development|SetHiddeninGame (Variables|Default|GetInteractWidget) true false))

(event Custom|OpenDoor
  (bind _asplayer_gamemode (Utilities|Casting|CastToPlayerGamemode (Game|GetGameMode)))
  (Variables|/Game/Game/Player/PlayerGamemode.PlayerGamemode_C|SetControlPanelUnlocked? _asplayer_gamemode true)
  (Variables|/Game/Game/Player/PlayerGamemode.PlayerGamemode_C|SetCurrentObjective _asplayer_gamemode 6))

(event EventBeginPlay)

(event Collision|EventActorBeginOverlap
  (params (OtherActor :type Actor%20Object%20Reference)))

(event EventTick
  (params (DeltaSeconds :type Float%20%28single-precision%29)))

(fn ConstructionScript)

(fn Interact
  (params (Interacting%20Entity :type Character%20Object%20Reference))
  (bind _asplayer_gamemode (Utilities|Casting|CastToPlayerGamemode (Game|GetGameMode)))
  (if (Variables|/Game/Game/Player/PlayerGamemode.PlayerGamemode_C|GetKey1? _asplayer_gamemode)
    (if (Variables|Default|GetInteracted?)
      (bind _returnvalue (UserInterface|CreateWidget "/Game/Game/Widgets/Hints/ControlPanel_AlreadyInteracted.ControlPanel_AlreadyInteracted_C"))
      (UserInterface|Viewport|AddtoViewport _returnvalue 0)
      (else
        (bind _returnvalue_2 (UserInterface|CreateWidget "/Game/Game/Widgets/Hints/Door_Unlocked.Door_Unlocked_C"))
        (UserInterface|Viewport|AddtoViewport _returnvalue_2 0)
        (Variables|Default|SetInteracted? true)
        (CallFunction|OpenDoor)
        (return false)))
    (else
      (bind _returnvalue_3 (UserInterface|CreateWidget "/Game/Game/Widgets/Hints/ControlPanel_KeyRequired.ControlPanel_KeyRequired_C"))
      (UserInterface|Viewport|AddtoViewport _returnvalue_3 0))))