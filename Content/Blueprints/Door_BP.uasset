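; Interactable double door Blueprint that swings its left and right leaves open and closed.
; Interact calls OpenDoor or CloseDoor based on IsOpen and always returns true.
; These events play or reverse one timeline, whose alpha lerps each leaf's yaw between its closed and open rotations.
; IsOpen flips only when the timeline finishes, in either direction.
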(event Custom|CloseDoor
  (bind _dooropenclose (Timeline|DoorOpenClose Reverse)
    (:Update
      (Transformation|SetRelativeRotation (Variables|Default|GetDoorRight) (Math|Rotator|MakeRotator 0.0 0.0 (Math|Float|Lerp (Variables|Default|GetDoorRightClosedRotation) (Variables|Default|GetDoorRightOpenRotation) _dooropenclose)) false false)
      (Transformation|SetRelativeRotation (Variables|Default|GetDoorLeft) (Math|Rotator|MakeRotator 0.0 0.0 (Math|Float|Lerp (Variables|Default|GetDoorLeftClosedRotation) (Variables|Default|GetDoorLeftOpenRotation) _dooropenclose)) false false))
    (:Finished
      (Variables|Default|SetIsOpen? (not (Variables|Default|GetIsOpen?))))))

(event Custom|OpenDoor
  (bind _dooropenclose (Timeline|DoorOpenClose Play)
    (:Update
      (Transformation|SetRelativeRotation (Variables|Default|GetDoorRight) (Math|Rotator|MakeRotator 0.0 0.0 (Math|Float|Lerp (Variables|Default|GetDoorRightClosedRotation) (Variables|Default|GetDoorRightOpenRotation) _dooropenclose)) false false)
      (Transformation|SetRelativeRotation (Variables|Default|GetDoorLeft) (Math|Rotator|MakeRotator 0.0 0.0 (Math|Float|Lerp (Variables|Default|GetDoorLeftClosedRotation) (Variables|Default|GetDoorLeftOpenRotation) _dooropenclose)) false false))
    (:Finished
      (Variables|Default|SetIsOpen? (not (Variables|Default|GetIsOpen?))))))

(fn ConstructionScript)

(fn Interact
  (params (Interacting%20Entity :type Character%20Object%20Reference))
  (if (not (Variables|Default|GetIsOpen?))
    (CallFunction|OpenDoor)
    (else
      (CallFunction|CloseDoor)))
  (return true))